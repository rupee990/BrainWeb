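; Dialog actor that turns to face the player and starts a conversation when the player walks into its trigger box.
; BeginPlay caches the player character, and Tick rotates the root with a look-at rotation toward it, offset -90 degrees in yaw.
; The box overlap casts the other actor to BP_PlayerCharacter and calls CreateDialog on it with the SimpleConversation asset from index 0.
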(event `self.ReceiveBeginPlay`
  (bind _returnvalue (`GameplayStatics.GetActorOfClass` "/Game/Blueprints/BP_PlayerCharacter.BP_PlayerCharacter_C"))
  (set `self.Player` _returnvalue))

(event `self.ReceiveTick`
  (params (DeltaSeconds :type "Float (single-precision)"))
  (bind (_returnvalue_roll _returnvalue_pitch _returnvalue_yaw) (`KismetMathLibrary.BreakRotator` (`KismetMathLibrary.FindLookAtRotation` (`self.K2_GetActorLocation`) (`self.K2_GetActorLocation` (`self.Player`)))))
  (`SceneComponent.K2_SetWorldRotation` (`self.DefaultSceneRoot`) (`KismetMathLibrary.MakeRotator` _returnvalue_roll _returnvalue_pitch (+ _returnvalue_yaw -90.0)) false false))

(event `self.Box.OnComponentBeginOverlap`
  (params (OverlappedComponent :type "PrimitiveComponent Object Reference") (OtherActor :type "Actor Object Reference") (OtherComp :type "PrimitiveComponent Object Reference") (OtherBodyIndex :type Integer) (bFromSweep :type Boolean) (SweepResult :type "HitResult Structure (by ref)"))
  (bind _asbp_player_character (cast `/Game/Blueprints/BP_PlayerCharacter` OtherActor))
  (`/Game/Blueprints/BP_PlayerCharacter.Create Dialog` _asbp_player_character "/Game/SimpleConversation.SimpleConversation" 0))

(fn `UserConstructionScript`)