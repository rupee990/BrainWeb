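; Player character Blueprint that hosts branching dialogue, running BrainWeb dialogue assets through an on-screen dialog box.
; CreateDialog binds the asset's start, node and end delegates, then starts it; NextNode and SetNextNode forward progression to it.
; Start and end events toggle UI-only input, cursor and the player controller's frozen flag.
; Executed nodes are cast by type to show a message, show query options, or remove the widget.
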(event `self.ReceiveBeginPlay`)

(event `OnStartDialog`
  (params (StartNode :type "BrainWebNode_Start Object Reference"))
  (bind _returnvalue (`GameplayStatics.GetPlayerController` 0))
  (bind _returnvalue_2 (`|CreateWidget` "/Game/Widgets/W_DialogBox.W_DialogBox_C" (`GameplayStatics.GetPlayerController` 0)))
  (set `self.DialogWidget` _returnvalue_2)
  (`UserWidget.AddToViewport` _returnvalue_2 0)
  (set `PlayerController.bShowMouseCursor` true _returnvalue)
  (set `PlayerController.bEnableClickEvents` true _returnvalue)
  (`WidgetBlueprintLibrary.SetInputMode_UIOnlyEx` _returnvalue _returnvalue_2)
  (bind _asbp_player_controller (cast `/Game/Blueprints/BP_PlayerController` _returnvalue))
  (set `/Game/Blueprints/BP_PlayerController.IsFrozen` true _asbp_player_controller))

(event `OnNodeExecute`
  (params (Node :type "BrainWebNode Object Reference") (Class :type "Object Class Reference"))
  (bind _asbrain_web_node_message (cast `BrainWebNode_Message` Node)
    (:`then`
      (`/Game/Widgets/W_DialogBox.SetMessage` (`self.DialogWidget`) (`BrainWebNode_Message.Message` _asbrain_web_node_message)))
    (:`CastFailed`
      (bind _asbrain_web_node_query (cast `BrainWebNode_Query` Node)
        (:`then`
          (`/Game/Widgets/W_DialogBox.SetQueries` (`self.DialogWidget`) (`BrainWebNode_Query.QuestionText` _asbrain_web_node_query) (`BrainWebNode_Query.Queries` _asbrain_web_node_query)))
        (:`CastFailed`
          (cast `BrainWebNode_End` Node)
          (`Widget.RemoveFromParent` (`self.DialogWidget`)))))))

(event `OnEndDialog`
  (params (EndNode :type "BrainWebNode_End Object Reference"))
  (bind _returnvalue (`GameplayStatics.GetPlayerController` 0))
  (set `PlayerController.bShowMouseCursor` false _returnvalue)
  (set `PlayerController.bEnableClickEvents` false _returnvalue)
  (`WidgetBlueprintLibrary.SetInputMode_GameOnly` _returnvalue)
  (bind _asbp_player_controller (cast `/Game/Blueprints/BP_PlayerController` _returnvalue))
  (set `/Game/Blueprints/BP_PlayerController.IsFrozen` false _asbp_player_controller))

(event `CustomEvent`
  (params (EndNode :type "BrainWebNode_End Object Reference")))

(fn `Create Dialog`
  (params (DiaglogAsset :type "BrainWebGraph Object Reference") (Index :type Integer))
  (set `self.CurrentDialog` DiaglogAsset)
  (add `BrainWebGraph.OnDialogueStartDelegate` DiaglogAsset (`|CreateDelegate` :!event `OnStartDialog`))
  (add `BrainWebGraph.OnNodeExecuteDelegate` DiaglogAsset (`|CreateDelegate` :!event `OnNodeExecute`))
  (add `BrainWebGraph.OnDialogueEndDelegate` DiaglogAsset (`|CreateDelegate` :!event `OnEndDialog`))
  (`BrainWebGraph.StartDialogue` (`self.CurrentDialog`) (`local.Index`)))

(fn `NextNode`
  (bind _currentdialog (`self.CurrentDialog`))
  (`/Engine/EditorBlueprintResources/StandardMacros.IsValid` _currentdialog
    (:`Is Valid`
      (`BrainWebGraph.NextNode` _currentdialog))))

(fn `SetNextNode`
  (params (NextNode :type "BrainWebNode Object Reference"))
  (bind _currentdialog (`self.CurrentDialog`))
  (`/Engine/EditorBlueprintResources/StandardMacros.IsValid` _currentdialog
    (:`Is Valid`
      (`BrainWebGraph.SetNextNode` _currentdialog NextNode))))

(fn `UserConstructionScript`)