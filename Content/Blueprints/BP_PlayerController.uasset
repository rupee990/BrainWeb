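; Player controller that turns movement and mouse axis inputs into walking and looking for the controlled pawn.
; Forward and right axes feed input vectors along the pawn's own axes into the BP_PlayerCharacter movement component, unless IsFrozen is set.
; Mouse axes drive controller yaw and pitch without checking IsFrozen, so looking stays active while movement is frozen.
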(event `InputAxis|MoveForward`
  (params (AxisValue :type "Float (single-precision)"))
  (bind _returnvalue (`self.K2_GetPawn`))
  (if (not (`self.IsFrozen`))
    (bind _asbp_player_character (cast `/Game/Blueprints/BP_PlayerCharacter` _returnvalue))
    (`PawnMovementComponent.AddInputVector` (`Character.CharacterMovement` _asbp_player_character) (* (`self.GetActorForwardVector` _returnvalue) AxisValue) false)))

(event `InputAxis|MoveRight`
  (params (AxisValue :type "Float (single-precision)"))
  (bind _returnvalue (`self.K2_GetPawn`))
  (if (not (`self.IsFrozen`))
    (bind _asbp_player_character (cast `/Game/Blueprints/BP_PlayerCharacter` _returnvalue))
    (`PawnMovementComponent.AddInputVector` (`Character.CharacterMovement` _asbp_player_character) (* (`self.GetActorRightVector` _returnvalue) AxisValue) false)))

(event `InputAxis|MouseX`
  (params (AxisValue :type "Float (single-precision)"))
  (`Pawn.AddControllerYawInput` (`self.K2_GetPawn`) AxisValue))

(event `InputAxis|MouseY`
  (params (AxisValue :type "Float (single-precision)"))
  (`Pawn.AddControllerPitchInput` (`self.K2_GetPawn`) AxisValue))

(fn `UserConstructionScript`)